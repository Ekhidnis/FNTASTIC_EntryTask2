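; Turtle spawner button that animates when triggered and then tells its referenced spawner to spawn.
; BeginPlay and the Activate event both enter a DoOnce, which records the Body's height, plays a sound and starts a timeline that offsets the Body vertically.
; When the timeline finishes, it calls Spawn on the spawner and resets the DoOnce, so activations during the animation are ignored.
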(event Custom|Activate
  (bind _body (Variables|Default|GetBody))
  (bind _returnvalue (Transformation|GetWorldLocation _body))
  ;[1 1 1] Animation + Sound
  (Utilities|FlowControl|DoOnce false :!label _label
    (:Completed
      (bind _output_get (Variables|Default|SetInitialLocZ (.z _returnvalue)))
      (Audio|PlaySoundatLocation "/Game/MobileStarterContent/Audio/Light02.Light02" (Math|Vector|MakeVector (.x _returnvalue) (.y _returnvalue) (.z _returnvalue)) "0, 0, 0" 0.2 4.0 0.0 0 0 0)
      (bind _animation (Timeline|ActivationAnim PlayFromStart)
        (:Update
          (Transformation|SetWorldLocation (Variables|Default|GetBody) (Math|Vector|MakeVector (.x _returnvalue) (.y _returnvalue) (+ _output_get _animation)) false false))
        (:Finished
          ;[1 1 1] Call Spawner
          (Default|Spawn (Variables|Default|GetTurtleSpawner_Spawner_Ref))
          (goto _label Reset))))))

(event EventBeginPlay
  (bind _body (Variables|Default|GetBody))
  (bind _returnvalue (Transformation|GetWorldLocation _body))
  ;[1 1 1] Animation + Sound
  (Utilities|FlowControl|DoOnce false :!label _label
    (:Completed
      (bind _output_get (Variables|Default|SetInitialLocZ (.z _returnvalue)))
      (Audio|PlaySoundatLocation "/Game/MobileStarterContent/Audio/Light02.Light02" (Math|Vector|MakeVector (.x _returnvalue) (.y _returnvalue) (.z _returnvalue)) "0, 0, 0" 0.2 4.0 0.0 0 0 0)
      (bind _animation (Timeline|ActivationAnim PlayFromStart)
        (:Update
          (Transformation|SetWorldLocation (Variables|Default|GetBody) (Math|Vector|MakeVector (.x _returnvalue) (.y _returnvalue) (+ _output_get _animation)) false false))
        (:Finished
          ;[1 1 1] Call Spawner
          (Default|Spawn (Variables|Default|GetTurtleSpawner_Spawner_Ref))
          (goto _label Reset))))))

(fn ConstructionScript)