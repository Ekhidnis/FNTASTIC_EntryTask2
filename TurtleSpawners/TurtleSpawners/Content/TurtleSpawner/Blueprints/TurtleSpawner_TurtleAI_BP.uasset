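; Turtle AI pawn that travels to a given destination actor, then explodes and removes itself.
; On BeginPlay, a looping timeline offsets the body's relative height from its current value for movement animation, and a fire effect attaches to the body.
; The Move event runs AI MoveTo, and on success attaches an explosion effect and destroys the actor after a short delay.
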(event Custom|Move
  (params (DestinationActor :type Turtle%20Spawner%20Loc%20BP%20Object%20Reference))
  ;[1 1 1] Lifespan
  (AI|AIMoveTo self "0, 0, 0" DestinationActor 1.0 false
    (:OnSuccess
      (Utilities|FlowControl|Sequence
        (:then_0
          ;[1 1 1] Effects
          (Effects|SpawnEmitterAttached "/Game/MobileStarterContent/Particles/P_Explosion.P_Explosion" (Variables|Default|GetBody) "None"))
        (:then_1
          (Utilities|FlowControl|Delay 1.0)
          (Actor|DestroyActor))))))

(event EventBeginPlay
  (bind _body (Variables|Default|GetBody))
  (bind _relativelocation (Variables|/Script/Engine.SceneComponent|GetRelativeLocation _body))
  (Utilities|FlowControl|Sequence
    (:then_0
      ;[1 1 1] Animation
      (bind _movementanim (Timeline|MovementAnim PlayFromStart)
        (:Update
          (Transformation|SetRelativeLocation (Variables|Default|GetBody) (Math|Vector|MakeVector (.x _relativelocation) (.y _relativelocation) (+ _movementanim (.z _relativelocation))) false false))
        (:Finished
          (Timeline|MovementAnim PlayFromStart))))
    (:then_1
      ;[1 1 1] Effects
      (Effects|SpawnEmitterAttached "/Game/MobileStarterContent/Particles/P_Fire.P_Fire" (Variables|Default|GetBody) "None" "0, 0, 0" "0, 0, 0" "1.000000,1.000000,1.000000" "KeepRelativeOffset" false))))

(fn ConstructionScript)