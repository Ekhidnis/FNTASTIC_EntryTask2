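; Interactable button that triggers a referenced turtle spawner when the first-person player presses the Action input nearby.
; Sphere overlap opens and closes a Gate, so the input only counts while the player is in range.
; Activation plays a sound and a timeline offsets the Body's height, then calls Spawn on the spawner when finished.
; A DoOnce blocks repeat presses until the animation completes.
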(event OnComponentBeginOverlap(Sphere)
  (params (OverlappedComponent :type Primitive%20Component%20Object%20Reference) (OtherActor :type Actor%20Object%20Reference) (OtherComp :type Primitive%20Component%20Object%20Reference) (OtherBodyIndex :type Integer) (bFromSweep :type Boolean) (SweepResult :type Hit%20Result%20Structure%20%28by%20ref%29))
  ;[1 1 1] Activation Range
  (Utilities|Casting|CastToFirstPersonCharacter OtherActor)
  (Utilities|FlowControl|Gate true) ; enters at Open
)

(event OnComponentEndOverlap(Sphere)
  (params (OverlappedComponent :type Primitive%20Component%20Object%20Reference) (OtherActor :type Actor%20Object%20Reference) (OtherComp :type Primitive%20Component%20Object%20Reference) (OtherBodyIndex :type Integer))
  ;[1 1 1] Activation Range
  (Utilities|Casting|CastToFirstPersonCharacter OtherActor)
  (Utilities|FlowControl|Gate true) ; enters at Close
)

(event Custom|Activate
  (bind _body (Variables|Default|GetBody))
  (bind _returnvalue (Transformation|GetWorldLocation _body))
  ;[1 1 1] Animation + Sound
  (Utilities|FlowControl|DoOnce false :!label _label
    (:Completed
      (bind _output_get (Variables|Default|SetInitialLocZ (.z _returnvalue)))
      (Audio|PlaySoundatLocation "/Game/MobileStarterContent/Audio/Light02.Light02" (Math|Vector|MakeVector (.x _returnvalue) (.y _returnvalue) (.z _returnvalue)) "0, 0, 0" 0.2 4.0 0.0 0 0 0)
      (bind _animation (Timeline|ActivationAnim PlayFromStart)
        (:Update
          (Transformation|SetWorldLocation (Variables|Default|GetBody) (Math|Vector|MakeVector (.x _returnvalue) (.y _returnvalue) (+ _output_get _animation)) false false))
        (:Finished
          ;[1 1 1] Call Spawner
          (Default|Spawn (Variables|Default|GetTurtleSpawner_Spawner_Ref))
          (goto _label Reset))))))

(event EventBeginPlay
  ;[1 1 1] Animation + Sound
)

(event Input|ActionEvents|InputActionAction
  (params (Key :type Key%20Structure :default "None"))
  ;[1 1 1] Activation Range
  (:Pressed
    (Utilities|FlowControl|Gate true
      (:Exit
        (CallFunction|Activate)))))

(fn ConstructionScript)